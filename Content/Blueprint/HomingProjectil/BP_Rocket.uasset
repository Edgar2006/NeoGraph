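; Homing rocket actor that drives a Niagara projectile effect and damages what it hits.
; Fire box-traces along the aim direction and passes the hit point, or trace end, to the effect as its aim position.
; The actor registers as the effect's callback handler, so exported particle positions trigger sphere traces that send DamageMessage to actors implementing BP_InteractInterace, then deactivate the effect.
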(event `self.ReceiveBeginPlay`
  (`NiagaraComponent.SetVariableObject` (`self.NS_HomingProjectil`) "BPCallbackHandler" self)
  (`ActorComponent.SetActive` (`self.NS_HomingProjectil`) false false))

(event `/Game/Blueprint/interface/BP_InteractInterace.Fire`
  (params (Start :type "Vector Structure") (Normal :type "Vector Structure"))
  (bind _endlocation (`self.BoxTrace` Start Normal 10000.0))
  (`ActorComponent.SetActive` (`self.NS_HomingProjectil`) true false)
  (`NiagaraComponent.SetVariableVec3` (`self.NS_HomingProjectil`) "aim_position" _endlocation))

(event `HitCollision`
  (params (Start :type "Vector Structure") (Normal :type "Vector Structure"))
  (bind _hitactorarr (`self.MultiSphareTrace` Start Normal 100.0))
  (for _array_element _hitactorarr
    (`self.CheckIsInterface` _array_element)))

(event `self.ReceiveParticleData`
  (params (Data :type "Array of BasicParticleData Structure (by ref)") (NiagaraSystem :type "NiagaraSystem Object Reference") (SimulationPositionOffset :type "Vector Structure (by ref)"))
  (for _array_element Data
    (`self.HitCollision` (`.Position` (break `BasicParticleData` _array_element)) (1.0 0.0 0.0)))
  (`ActorComponent.SetActive` (`self.NS_HomingProjectil`) false false))

(fn `BoxTrace`
  (params (Start :type "Vector Structure") (Normal :type "Vector Structure") (B :type "Float (double-precision)"))
  (returns (EndLocation :type "Vector Structure"))
  (bind _returnvalue (+ Start (* Normal B)))
  (bind _outhit (`KismetSystemLibrary.BoxTraceSingle` :`Start` Start :`End` _returnvalue :`HalfSize` (50.0 50.0 50.0) :`TraceChannel` "TraceTypeQuery1" :`DrawDebugType` "ForDuration"))
  (bind (_bblockinghit _binitialoverlap _time _distance _location) (`GameplayStatics.BreakHitResult` _outhit))
  (if _bblockinghit
    (return _location)
    (else
      (return _returnvalue))))

(fn `CheckIsInterface`
  (params (hitActor :type "Actor Object Reference"))
  (if (`KismetSystemLibrary.DoesImplementInterface` hitActor "/Game/Blueprint/interface/BP_InteractInterace.BP_InteractInterace_C")
    (message `/Game/Blueprint/interface/BP_InteractInterace.Damage` hitActor)))

(fn `MultiSphareTrace`
  (params (Start :type "Vector Structure") (Normal :type "Vector Structure") (Radius :type "Float (double-precision)"))
  (returns (HitActorArr :type "Array of Actor Object Reference"))
  (locals (HitActor :type "Array of Actor Object Reference"))
  (bind _outhits (`KismetSystemLibrary.SphereTraceMulti` Start (+ Start (* Normal Radius)) Radius "TraceTypeQuery3"))
  (for _array_element _outhits
    (`KismetArrayLibrary.Array_Add` (`local.HitActor`) (`.HitActor` (`GameplayStatics.BreakHitResult` _array_element))))
  (return (`local.HitActor`)))

(fn `UserConstructionScript`)